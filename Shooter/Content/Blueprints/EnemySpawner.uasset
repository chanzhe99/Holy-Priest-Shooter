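; Enemy spawner actor that spawns a knight enemy with a melee behavior tree at its own transform.
; A Delay on Tick acts as a repeating two-second timer, with no spawn limit.
; The first spawn caches the knight's scaled capsule half-height, prints a debug string and lifts that knight by the offset.
; Later spawns apply the cached offset directly to the spawn location.
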(event Collision|EventActorBeginOverlap
  (params (OtherActor :type Actor%20Object%20Reference)))

(event EventTick
  (params (DeltaSeconds :type Float%20%28single-precision%29))
  (Utilities|FlowControl|Delay 2.0)
  (bind _returnvalue (AI|SpawnAIFromClass "/Game/Blueprints/EnemyAI/Enemy_KnightBase.Enemy_KnightBase_C" "/Game/Blueprints/EnemyAI/Enemy_MeleeBT.Enemy_MeleeBT" (+ (Transformation|GetActorLocation) (Variables|Default|GetEnemyHalfHeight)) (Transformation|GetActorRotation) false 0))
  (if (Math|Vector|VectorIsZero (Variables|Default|GetEnemyHalfHeight))
    (Development|PrintString "Hello")
    (bind _asenemy_knight_base (Utilities|Casting|CastToEnemy_KnightBase _returnvalue))
    (bind _output_get (Variables|Default|SetEnemyHalfHeight (Math|Vector|MakeVector 0.0 0.0 (Components|Capsule|GetScaledCapsuleHalfHeight (Variables|/Script/Engine.Character|GetCapsuleComponent _asenemy_knight_base)))))
    (Transformation|SetActorLocation _asenemy_knight_base (+ _output_get (Transformation|GetActorLocation)) false false)))

(fn ConstructionScript)