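; HolyWater is an area-of-effect actor that applies a holy water status to knight enemies.
; On actor overlap, it flags every Enemy_KnightBase inside its AOESphere as HolyWatered, swaps that enemy's first mesh material and prints the flag for debugging.
; If the sphere contains any knights, the actor sets a short lifespan so it destroys itself shortly afterward.
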(event Collision|EventActorBeginOverlap
  (params (OtherActor :type Actor%20Object%20Reference))
  (bind _aoe_sphere (Variables|Default|GetAOE%20Sphere))
  (bind _overlappingactors (Collision|GetOverlappingActors _aoe_sphere "/Game/Blueprints/EnemyAI/Enemy_KnightBase.Enemy_KnightBase_C" :!class /Script/Engine.PrimitiveComponent))
  (for _array_element _overlappingactors
    (bind _asenemy_knight_base (Utilities|Casting|CastToEnemy_KnightBase _array_element))
    (bind _output_get (Variables|/Game/Blueprints/EnemyAI/Enemy_KnightBase.Enemy_KnightBase_C|SetHolyWatered _asenemy_knight_base true))
    (Utilities|FlowControl|Sequence
      (:then_0
        (Development|PrintString (Utilities|String|ToString(Boolean) _output_get)))
      (:then_1
        (Rendering|Material|SetMaterial (Variables|/Script/Engine.Character|GetMesh _asenemy_knight_base) 0 "/Engine/MapTemplates/Materials/BasicAsset01.BasicAsset01"))))
  (if (> (Utilities|Array|Length _overlappingactors) 0)
    (Actor|SetLifeSpan 0.3)))

(fn ConstructionScript)