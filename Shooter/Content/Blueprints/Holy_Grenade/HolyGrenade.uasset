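; Holy grenade actor that detonates on a fixed fuse timer started at BeginPlay.
; Detonation activates the particle system, fires a radial force impulse, destroys the static mesh and plays the Explosion2 component.
; A short life span set at detonation keeps the actor alive for the effects before it is removed.
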(event Custom|Detonate
  (Utilities|FlowControl|Sequence
    (:then_0
      (Components|Activation|Activate (Variables|Default|GetParticleSystem) false)
      (Actor|SetLifeSpan 2.5))
    (:then_1
      (Class|RadialForceComponent|FireImpulse (Variables|Default|GetRadialForce))
      (Components|DestroyComponent (Variables|Default|GetStaticMesh)))
    (:then_2
      (Audio|Components|Audio|Play (Variables|Default|Getexplosion_2) 0.0))))

(event EventBeginPlay
  (Utilities|Time|SetTimerbyEvent (delegate Custom|Detonate) 2.0))

(fn ConstructionScript)